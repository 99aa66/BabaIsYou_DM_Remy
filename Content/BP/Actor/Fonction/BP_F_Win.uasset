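; BP_F_Win is a function actor that switches the win condition of a set of pawns on or off.
; Its Activate and Desactivate events loop over PawnArray, setting each pawn's WinCondition to true or false respectively.
; Each event then prints a debug string, and the construction script only calls its parent.
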(event EventActivate
  (for _array_element (Variables|Default|GetPawn_Array)
    (Variables|/Game/BP/Base_Actor/BP_Player.BP_Player_C|SetWin%20Condition _array_element true))
  (Development|PrintString "Win"))

(event EventDesactivate
  (for _array_element (Variables|Default|GetPawn_Array)
    (Variables|/Game/BP/Base_Actor/BP_Player.BP_Player_C|SetWin%20Condition _array_element false))
  (Development|PrintString "Desactivate"))

(fn ConstructionScript
  (|CallParentFunction))