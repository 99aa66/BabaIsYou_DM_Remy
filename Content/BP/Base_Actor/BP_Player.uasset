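; BP_Player is a player actor that ends the game when it hits another BP_Player while WinCondition is true.
; On BeginPlay it disables collision on its capsule, and a pair of custom events switches that collision off or back to query and physics.
; The capsule's hit event casts the other actor to BP_Player, checks WinCondition and quits the application.
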(event OnComponentHit(CapsuleComponent)
  (params (HitComponent :type Primitive%20Component%20Object%20Reference) (OtherActor :type Actor%20Object%20Reference) (OtherComp :type Primitive%20Component%20Object%20Reference) (NormalImpulse :type Vector :default "0, 0, 0") (Hit :type Hit%20Result%20Structure%20%28by%20ref%29))
  (Utilities|Casting|CastToBP_Player OtherActor)
  (if (Variables|Default|GetWin%20Condition)
    (Game|QuitGame 0 "Quit" false)))

(event Custom|No_More_Collision
  (Collision|SetCollisionEnabled (Variables|Collision|GetCapsuleComponent) "NoCollision"))

(event Custom|Add_Collision
  (Collision|SetCollisionEnabled (Variables|Collision|GetCapsuleComponent) "QueryAndPhysics"))

(event EventBeginPlay
  (CallFunction|NoMoreCollision))

(fn ConstructionScript)